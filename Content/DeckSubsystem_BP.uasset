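; Satisfactory mod subsystem that builds name lookups for control deck features and exports game icons as PNGs.
; On BeginPlay it maps customization descriptors and swatches by display name, plus quick-action labels to keys.
; Separate events export action, blueprint, building, customizer and resource icons to SFControlPanelIcons in the project directory.
; Each exporter draws textures through a dynamic material onto a reused render target, discovering most sources by native class search.
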(event `self.ReceiveBeginPlay`
  (`self.InitCustomizerDescriptors`)
  (`self.InitSwatchDescriptors`)
  (`self.InitAction`))

(event `self.ActionIconExtractor`
  (`self.ActionIcons`))

(event `self.BlueprintIconExtraction_BIE`
  (`self.BlueprintIcons`))

(event `self.RecipeIconExtraction_BIE`
  (`self.BuildableIcons`))

(event `self.CustomizerIconExtractor`
  (`self.CustomizerIcons`))

(event `self.ResourceIconExtractor`
  (`self.ItemIcons`))

(fn `ActionIcons`
  (bind _map (`|MakeMap` "build" "/Game/FactoryGame/Interface/UI/Assets/HUD_Elements/Keybord_Shortcuts/IconDesc_BuildGun.IconDesc_BuildGun" "codex" "/Game/FactoryGame/Interface/UI/Assets/HUD_Elements/Keybord_Shortcuts/IconDesc_Codex.IconDesc_Codex" "paint" "/Game/FactoryGame/Interface/UI/Assets/HUD_Elements/Keybord_Shortcuts/IconDesc_Customizer.IconDesc_Customizer" "dismantle" "/Game/FactoryGame/Interface/UI/Assets/HUD_Elements/Keybord_Shortcuts/IconDesc_Dismantle.IconDesc_Dismantle" "flashlight" "/Game/FactoryGame/Interface/UI/Assets/HUD_Elements/Keybord_Shortcuts/IconDesc_Flashlight.IconDesc_Flashlight" "holster" "/Game/FactoryGame/Interface/UI/Assets/HUD_Elements/Keybord_Shortcuts/IconDesc_Holster.IconDesc_Holster" "inventory" "/Game/FactoryGame/Interface/UI/Assets/HUD_Elements/Keybord_Shortcuts/IconDesc_Inventory.IconDesc_Inventory" "map" "/Game/FactoryGame/Interface/UI/Assets/HUD_Elements/Keybord_Shortcuts/IconDesc_Map.IconDesc_Map" "camera" "/Game/FactoryGame/Interface/UI/Assets/MonochromeIcons/TXUI_MIcon_Pioneer.TXUI_MIcon_Pioneer" "thirdperson" "/Game/FactoryGame/Interface/UI/Assets/MonochromeIcons/TXUI_MIcon_Pioneer.TXUI_MIcon_Pioneer" :!valuetype "Texture2D Object Reference"))
  (bind _returnvalue (`KismetMaterialLibrary.CreateDynamicMaterialInstance` "/SFControlPanel/IconSystem/MM_RenderMaterial.MM_RenderMaterial"))
  (bind _returnvalue_2 (`KismetRenderingLibrary.CreateRenderTarget2D` 512 512 "RTF_RGBA8" (struct :`A` 1.0) false true))
  (bind _keys (`BlueprintMapLibrary.Map_Keys` _map))
  (for _array_element _keys
    (`KismetRenderingLibrary.ClearRenderTarget2D` _returnvalue_2 (struct))
    (`MaterialInstanceDynamic.SetTextureParameterValue` _returnvalue "Texture" (`BlueprintMapLibrary.Map_Find` _map _array_element))
    (`KismetRenderingLibrary.DrawMaterialToRenderTarget` _returnvalue_2 _returnvalue)
    (`KismetRenderingLibrary.ExportRenderTarget` _returnvalue_2 (`KismetStringLibrary.Concat_StrStr` (`KismetSystemLibrary.GetProjectDirectory`) "SFControlPanelIcons/") (`KismetStringLibrary.Concat_StrStr` _array_element ".png")))
  (`KismetRenderingLibrary.ReleaseRenderTarget2D` _returnvalue_2))

(fn `BlueprintIcons`
  (bind _returnvalue (`KismetMaterialLibrary.CreateDynamicMaterialInstance` "/SFControlPanel/IconSystem/MM_RenderMaterial.MM_RenderMaterial"))
  (bind _returnvalue_2 (`KismetRenderingLibrary.CreateRenderTarget2D` 512 512 "RTF_RGBA8" (struct :`A` 1.0) false true))
  (bind _out_descriptors (`FGBlueprintSubsystem.GetBlueprintDescriptors` (`FGBlueprintSubsystem.GetBlueprintSubsystem` self) self))
  (for _array_element _out_descriptors
    (`KismetRenderingLibrary.ClearRenderTarget2D` _returnvalue_2 (struct))
    (`MaterialInstanceDynamic.SetTextureParameterValue` _returnvalue "Texture" (`FGItemDescriptor.mPersistentBigIcon` _array_element))
    (`KismetRenderingLibrary.DrawMaterialToRenderTarget` _returnvalue_2 _returnvalue)
    (`KismetRenderingLibrary.ExportRenderTarget` _returnvalue_2 (`KismetStringLibrary.Concat_StrStr` (`KismetSystemLibrary.GetProjectDirectory`) "SFControlPanelIcons/") (`KismetStringLibrary.Concat_StrStr` (break `BlueprintRecord` (`FGBlueprintDescriptor.GetDescriptorAsRecord` _array_element)) ".png")))
  (`KismetRenderingLibrary.ReleaseRenderTarget2D` _returnvalue_2))

(fn `BuildableIcons`
  (bind _returnvalue (`KismetMaterialLibrary.CreateDynamicMaterialInstance` "/SFControlPanel/IconSystem/MM_RenderMaterial.MM_RenderMaterial"))
  (bind _returnvalue_2 (`KismetRenderingLibrary.CreateRenderTarget2D` 512 512 "RTF_RGBA8" (struct :`A` 1.0) false true))
  (bind _foundclasses (`BlueprintAssetHelperLibrary.FindNativeClassesByType` "/Script/FactoryGame.FGBuildingDescriptor"))
  (for _array_element _foundclasses
    (bind _asfgbuilding_descriptor (castclass `FGBuildingDescriptor` _array_element))
    (if true
      (`KismetRenderingLibrary.ClearRenderTarget2D` _returnvalue_2 (struct))
      (`MaterialInstanceDynamic.SetTextureParameterValue` _returnvalue "Texture" (`FGItemDescriptor.mPersistentBigIcon` (`BlueprintReflectionLibrary.GetClassDefaultObject` _asfgbuilding_descriptor)))
      (`KismetRenderingLibrary.DrawMaterialToRenderTarget` _returnvalue_2 _returnvalue)
      (`KismetRenderingLibrary.ExportRenderTarget` _returnvalue_2 (`KismetStringLibrary.Concat_StrStr` (`KismetSystemLibrary.GetProjectDirectory`) "SFControlPanelIcons/") (`KismetStringLibrary.Concat_StrStr` (`KismetSystemLibrary.GetClassDisplayName` _asfgbuilding_descriptor) ".png"))))
  (`KismetRenderingLibrary.ReleaseRenderTarget2D` _returnvalue_2))

(fn `CustomizerIcons`
  (bind _returnvalue (`KismetMaterialLibrary.CreateDynamicMaterialInstance` "/SFControlPanel/IconSystem/MM_RenderMaterial.MM_RenderMaterial"))
  (bind _returnvalue_2 (`KismetRenderingLibrary.CreateRenderTarget2D` 512 512 "RTF_RGBA8" (struct :`A` 1.0) false true))
  (bind _foundclasses (`BlueprintAssetHelperLibrary.FindNativeClassesByType` "/Script/FactoryGame.FGCustomizationRecipe"))
  (for _array_element _foundclasses
    (bind _asfgcustomization_recipe (castclass `FGCustomizationRecipe` _array_element))
    (`KismetRenderingLibrary.ClearRenderTarget2D` _returnvalue_2 (struct))
    (bind _returnvalue_3 (`FGCustomizationRecipe.GetCustomizationDescriptor` _asfgcustomization_recipe))
    (`MaterialInstanceDynamic.SetTextureParameterValue` _returnvalue "Texture" (`FGBlueprintFunctionLibrary.GetIconForCustomizationDesc` _returnvalue_3))
    (`KismetRenderingLibrary.DrawMaterialToRenderTarget` _returnvalue_2 _returnvalue)
    (`self.ExportRenderTarget_SCP` _returnvalue_2 (`KismetSystemLibrary.GetClassDisplayName` _returnvalue_3)))
  (`KismetRenderingLibrary.ReleaseRenderTarget2D` _returnvalue_2))

(fn `ExportRenderTarget_SCP`
  (params (TextureRenderTarget :type "TextureRenderTarget2D Object Reference") (ObjectName :type String))
  (`KismetRenderingLibrary.ExportRenderTarget` TextureRenderTarget (`KismetStringLibrary.Concat_StrStr` (`KismetSystemLibrary.GetProjectDirectory`) "SFControlPanelIcons/") (`KismetStringLibrary.Concat_StrStr` ObjectName ".png")))

(fn `InitAction`
  (set `self.QuickActions` (`|MakeMap` "Build Gun" "build" "Dismantle" "dismantle" "Customizer" "paint" "Holster" "holster" "Inventory" "inventory" "Photo Mode" "camera" "Third-Person" "thirdperson")))

(fn `InitCustomizerDescriptors`
  (bind _customizationdescriptors (`self.CustomizationDescriptors`))
  (bind _foundclasses (`BlueprintAssetHelperLibrary.FindNativeClassesByType` "/Script/FactoryGame.FGCustomizationRecipe"))
  (for _array_element _foundclasses
    (bind _returnvalue (`FGCustomizationRecipe.GetCustomizationDescriptor` (castclass `FGCustomizationRecipe` _array_element :!pure true)))
    (castclass `FGFactoryCustomizationDescriptor_Swatch` _returnvalue
      (:`CastFailed`
        (`BlueprintMapLibrary.Map_Add` _customizationdescriptors (`KismetSystemLibrary.GetClassDisplayName` _returnvalue) _returnvalue))))
  (`BlueprintLoggingLibrary.LogWarning` (`KismetStringLibrary.Concat_StrStr` "UFGCustomizationRecipe: " (`KismetStringLibrary.Conv_IntToString` (`BlueprintMapLibrary.Map_Length` _customizationdescriptors)))))

(fn `InitSwatchDescriptors`
  (bind _swatchdescriptors (`self.SwatchDescriptors`))
  (bind _foundclasses (`BlueprintAssetHelperLibrary.FindNativeClassesByType` "/Script/FactoryGame.FGFactoryCustomizationDescriptor_Swatch"))
  (for _array_element _foundclasses
    (bind _asfgfactory_customization_descriptor_swatch (castclass `FGFactoryCustomizationDescriptor_Swatch` _array_element))
    (`BlueprintMapLibrary.Map_Add` _swatchdescriptors (`KismetSystemLibrary.GetClassDisplayName` _asfgfactory_customization_descriptor_swatch) _asfgfactory_customization_descriptor_swatch))
  (`BlueprintLoggingLibrary.LogWarning` (`KismetStringLibrary.Concat_StrStr` "UFGFactoryCustomizationDescriptor_Swatch: : " (`KismetStringLibrary.Conv_IntToString` (`BlueprintMapLibrary.Map_Length` _swatchdescriptors)))))

(fn `ItemIcons`
  (bind _returnvalue (`KismetMaterialLibrary.CreateDynamicMaterialInstance` "/SFControlPanel/IconSystem/MM_RenderMaterial.MM_RenderMaterial"))
  (bind _returnvalue_2 (`KismetRenderingLibrary.CreateRenderTarget2D` 512 512 "RTF_RGBA8" (struct :`A` 1.0) false true))
  (bind _foundclasses (`BlueprintAssetHelperLibrary.FindNativeClassesByType` "/Script/FactoryGame.FGResourceDescriptor"))
  (for _array_element _foundclasses
    (bind _asfgitem_descriptor (castclass `FGItemDescriptor` _array_element))
    (if (not (`KismetArrayLibrary.Array_Contains` (`|MakeArray` "/Game/FactoryGame/Equipment/Trinkets/Desc_Trinket_Alpaca.Desc_Trinket_Alpaca_C" "/Game/FactoryGame/Resource/Parts/VolcanicGas/Desc_VolcanicGas.Desc_VolcanicGas_C" "/Game/FactoryGame/Resource/Parts/SuperFuelRod/Desc_SuperFuelRod.Desc_SuperFuelRod_C" "/Game/FactoryGame/Resource/Parts/HydrogenGas/Desc_HydrogenGas.Desc_HydrogenGas_C" :!type "FGItemDescriptor Class Reference") _asfgitem_descriptor))
      (`KismetRenderingLibrary.ClearRenderTarget2D` _returnvalue_2 (struct))
      (`MaterialInstanceDynamic.SetTextureParameterValue` _returnvalue "Texture" (`FGItemDescriptor.mPersistentBigIcon` (`BlueprintReflectionLibrary.GetClassDefaultObject` _asfgitem_descriptor)))
      (`KismetRenderingLibrary.DrawMaterialToRenderTarget` _returnvalue_2 _returnvalue)
      (`KismetRenderingLibrary.ExportRenderTarget` _returnvalue_2 (`KismetStringLibrary.Concat_StrStr` (`KismetSystemLibrary.GetProjectDirectory`) "SFControlPanelIcons/") (`KismetStringLibrary.Concat_StrStr` (`KismetSystemLibrary.GetClassDisplayName` _asfgitem_descriptor) ".png"))))
  (`KismetRenderingLibrary.ReleaseRenderTarget2D` _returnvalue_2))

(fn `UserConstructionScript`)